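; Player Blueprint that moves its capsule along a circular path, driven by the A and D keys.
; A hold macro loops on a Speed delay until release, and its completion feeds a movement calculation into MoveComponentTo.
; That calculation builds a fixed-height target from cosine and sine expressions.
; A separate setup graph picks radius, X offset and item meshes for Mummy or other character types.
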(event `self.ReceiveBeginPlay`
  ;[1 1 1] Input from User
  (`self.EnableInput` (`GameplayStatics.GetPlayerController` 0)))

(event `Key|A`
  (params (Key :type "Key Structure"))
  ;[1 1 1] Move
  (:`Pressed`
    (`self.Set Value` Key :!label _label
      (:`Complete`
        (bind _returnvalue (`self.Calculate_Movement` :!label _label_2)
          (:`Complete`
            (`KismetSystemLibrary.MoveComponentTo` (`self.CapsuleComponent`) _returnvalue (struct) false false (`self.speed`)))))))
  (:`Released`
    (goto _label :!via `Releas`)))

(event `Key|D`
  (params (Key :type "Key Structure"))
  ;[1 1 1] Move
  (:`Pressed`
    (`self.Set Value` Key :!label _label_3
      (:`Complete`
        (goto _label_2))))
  (:`Released`
    (goto _label_3 :!via `Releas`)))

(fn `UserConstructionScript`)
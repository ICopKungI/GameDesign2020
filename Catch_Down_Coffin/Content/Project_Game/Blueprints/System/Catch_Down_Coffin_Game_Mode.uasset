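; Game mode for the Catch Down Coffin level, running the match countdown and scattering the course's pickups and obstacles.
; On BeginPlay, Start_Game resets match state and starts a one-second looping timer that opens Mummy_Win when time runs out.
; A loop then steps along X from a TargetPoint at fixed spacing, spawning randomly offset and yawed cacti, with a larger item box every ItemFrequency steps.
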(event `Timmer`
  ;[1 1 1] Timmer
  (if (and (!= 0 (`self.Time`)) (not (`self.Game_Over`)))
    (set `self.Time` (- (`self.Time`) 1))
    (if (== 0 (`self.Time`))
      (set `self.Game_Over` true)
      (set `self.Who_Win` true)
      (`KismetSystemLibrary.K2_ClearTimer` null "Timmer")
      (`GameplayStatics.OpenLevel` "Mummy_Win"))))

(event `self.ReceiveBeginPlay`
  ;[1 1 1] Set Game When Start
  (`self.Start_Game`
    (:`Complete`
      (bind _returnvalue (`GameplayStatics.GetActorOfClass` "/Script/Engine.TargetPoint"))
      (for _index (range 1 (+ (+ (`KismetMathLibrary.FTrunc` (/ (`self.length`) (`self.Distance`))) 1) 1))
        (if (== (mod _index (`self.Item_frequency`)) 0)
          (set `self.Scale` (2.5 2.5 2.5))
          (bind _returnvalue_2 (`self.GetTransform` _returnvalue))
          (bind _returnvalue_3 (`KismetMathLibrary.MakeTransform` (+ (.location _returnvalue_2) (`KismetMathLibrary.MakeVector` (* _index (`self.Distance`)) (`KismetMathLibrary.RandomFloatInRange` 0.0 (`self.Width`)) 50.0)) (`KismetMathLibrary.MakeRotator` (.roll (.rotation _returnvalue_2)) (.pitch (.rotation _returnvalue_2)) (`KismetMathLibrary.RandomFloatInRange` 0.0 359.0)) (`self.Scale`)))
          (`|SpawnActorFromClass` "/Game/Project_Game/Blueprints/Item/Item_Box1.Item_Box1_C" _returnvalue_3 "Undefined" "OverrideRootScale" null null)
          (else
            (set `self.Scale` (1.75 1.75 1.75))
            (`|SpawnActorFromClass` (`|GetArrayItem` (`|MakeArray` "/Game/Project_Game/Blueprints/Obstruction/Cactus.Cactus_C" :!type "Actor Class Reference") (`KismetMathLibrary.RandomIntegerInRange` 0)) _returnvalue_3 "Undefined" "OverrideRootScale" null null)))))))

(fn `UserConstructionScript`)
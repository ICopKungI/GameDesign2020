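; Poison item projectile that reverses the movement direction of the character it hits.
; On BeginPlay it takes its static mesh from the item array on the Catch Down Coffin game mode.
; On hitting a ThirdPersonCharacter3, it sets that character's reverse-direction flag and switch timer, then destroys itself.
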(event `self.ReceiveBeginPlay`
  ;[1 1 1] Set StaticMesh Item
  (bind _ascatch_down_coffin_game_mode (cast `/Game/Project_Game/Blueprints/System/Catch_Down_Coffin_Game_Mode` (`GameplayStatics.GetGameMode`)))
  (`StaticMeshComponent.SetStaticMesh` (`self.StaticMesh`) (`|GetArrayItem` (`/Game/Project_Game/Blueprints/System/Catch_Down_Coffin_Game_Mode.Item_Of_Mummy` _ascatch_down_coffin_game_mode) 1)))

(event `self.ReceiveHit`
  (params (MyComp :type "PrimitiveComponent Object Reference") (Other :type "Actor Object Reference") (OtherComp :type "PrimitiveComponent Object Reference") (bSelfMoved :type Boolean) (HitLocation :type "Vector Structure") (HitNormal :type "Vector Structure") (NormalImpulse :type "Vector Structure") (Hit :type "HitResult Structure (by ref)"))
  ;[1 1 1] The coffin was poisoned.
  (bind _asthird_person_character_3 (cast `/Game/Project_Game/Blueprints/Player/ThirdPersonCharacter3` Other))
  (set `/Game/Project_Game/Blueprints/Player/ThirdPersonCharacter3.Reverse direction` true _asthird_person_character_3)
  (set `/Game/Project_Game/Blueprints/Player/ThirdPersonCharacter3.Time_Switch` 3.0 _asthird_person_character_3)
  (`self.K2_DestroyActor`) ; Then destroy this projectile
)

(fn `UserConstructionScript`)
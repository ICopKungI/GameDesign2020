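; Item box for Catch Down Coffin that awards a random role-specific item when hit by one of the three player characters.
; On Hit, it reads whether the player is Mummy or Coffin and gates repeat hits by comparing SelfMoved to a Status flag.
; Macros pick from the GameMode's item meshes, reskin the cube and store the item name in the GameMode.
; The cube then jumps upward and is destroyed after a short delay.
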(event `self.ReceiveBeginPlay`
  ;[1 1 1] Set Object
  (bind _ascatch_down_coffin_game_mode (cast `/Game/Project_Game/Blueprints/System/Catch_Down_Coffin_Game_Mode` (`GameplayStatics.GetGameMode`)))
  (set `self.Game_Mode` _ascatch_down_coffin_game_mode))

(event `self.ReceiveHit`
  (params (MyComp :type "PrimitiveComponent Object Reference") (Other :type "Actor Object Reference") (OtherComp :type "PrimitiveComponent Object Reference") (bSelfMoved :type Boolean) (HitLocation :type "Vector Structure") (HitNormal :type "Vector Structure") (NormalImpulse :type "Vector Structure") (Hit :type "HitResult Structure (by ref)"))
  ;[1 1 1] Item Box
  (bind _asthird_person_character_1 (cast `/Game/Project_Game/Blueprints/Player/ThirdPersonCharacter1` Other)
    (:`then`
      (set `self.mummy_or_coffin` (`/Game/Project_Game/Blueprints/Player/ThirdPersonCharacter1.Type_Player` _asthird_person_character_1)))
    (:`CastFailed`
      (bind _asthird_person_character_2 (cast `/Game/Project_Game/Blueprints/Player/ThirdPersonCharacter2` Other)
        (:`then`
          (set `self.mummy_or_coffin` (`/Game/Project_Game/Blueprints/Player/ThirdPersonCharacter2.Type_Player` _asthird_person_character_2)))
        (:`CastFailed`
          (bind _asthird_person_character_3 (cast `/Game/Project_Game/Blueprints/Player/ThirdPersonCharacter3` Other))
          (set `self.mummy_or_coffin` (`/Game/Project_Game/Blueprints/Player/ThirdPersonCharacter3.Type_Player` _asthird_person_character_3))))))
  (`self.Set_Item_Player` bSelfMoved
    (:`HIt`
      (set `self.status` true)
      (`self.Show_Item`
        (:`Complete`
          (set `self.status` false))))))

(fn `UserConstructionScript`)